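; Base-style projectile Blueprint for ARPG weapons that delivers Gameplay Ability System damage on box overlap.
; Overlaps ignore the instigator and resolve only on the server, adding the hit result to the damage spec's context before applying it to the hit character's ability system.
; The projectile destroys itself on static geometry, non-character hits or successful damage application.
; Destruction spawns a random impact emitter at its transform.
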(event OnComponentBeginOverlap(BoxComponent)
  (params (OverlappedComponent :type Primitive%20Component%20Object%20Reference) (OtherActor :type Actor%20Object%20Reference) (OtherComp :type Primitive%20Component%20Object%20Reference) (OtherBodyIndex :type Integer) (bFromSweep :type Boolean) (SweepResult :type Hit%20Result%20Structure%20%28by%20ref%29))
  (bind _damageeffectspechandle (Variables|Default|GetDamageEffectSpecHandle))
  (if (!= OtherActor (Game|GetInstigator))
    (Networking|SwitchHasAuthority
      (:Authority
        (if (Utilities|Enum|Equal(Enum) (Variables|/Script/Engine.SceneComponent|GetMobility OtherComp) "Static")
          (Actor|DestroyActor)
          (else
            (bind _asarpgcharacter (Utilities|Casting|CastToARPGCharacter OtherActor)
              (:then
                (Utilities|IsValid (Ability|GetAbilitySystemComponent _asarpgcharacter)
                  (:Is%20Valid
                    (bind _returnvalue (Class|AbilitySystemBlueprintLibrary|GetEffectContext _damageeffectspechandle))
                    (Class|AbilitySystemBlueprintLibrary|EffectContextAddHitResult _returnvalue SweepResult false)
                    (GameplayEffects|ApplyGameplayEffectSpecToSelf (Ability|GetAbilitySystemComponent _asarpgcharacter) _damageeffectspechandle)
                    (Actor|DestroyActor))))
              (:CastFailed
                (Actor|DestroyActor)))))))))

(event Custom|OnDestroyed_Event
  (params (DestroyedActor :type Actor%20Object%20Reference))
  (bind _returnvalue (Transformation|GetActorTransform DestroyedActor))
  (Effects|SpawnEmitteratLocation (.OutItem (Utilities|Array|Random (Variables|Default|GetImpactEffects))) (.location _returnvalue) (.rotation _returnvalue)))

(event EventBeginPlay
  (|CallParentFunction)
  (Game|AssignOnDestroyed (delegate Custom|OnDestroyed_Event)))

(fn ConstructionScript)