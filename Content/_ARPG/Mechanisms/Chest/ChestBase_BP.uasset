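; Base chest mechanism that a pawn can open once through Interact.
; Interact passes through a DoOnce, then calls Open and returns true.
; Open sets Triggered, plays a timeline that rolls AdditiveMesh from closed to -90 degrees, and calls PlaySound to play the sound at the chest's location.
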(event Custom|Open
  (Variables|Default|SetbTriggered true)
  (Utilities|FlowControl|Sequence
    (:then_0
      (bind _alpha (Timeline|Timeline_Open PlayFromStart)
        (:Update
          (Transformation|SetRelativeRotation (Variables|Default|GetAdditiveMesh) (Math|Rotator|MakeRotator (Math|Float|Lerp 0.0 -9e+01 _alpha) 0.0 0.0) false false))))
    (:then_1
      (CallFunction|PlaySound))))

(event Custom|PlaySound
  (Audio|PlaySoundatLocation (Variables|Default|GetSound) (Transformation|GetActorLocation) "0, 0, 0" 0.5 1.0 0.0 0 0 0 0))

(event EventBeginPlay)

(event Collision|EventActorBeginOverlap
  (params (OtherActor :type Actor%20Object%20Reference)))

(event EventTick
  (params (DeltaSeconds :type Float%20%28single-precision%29)))

(fn ConstructionScript)

(fn Interact
  (params (InstigatorPawn :type Pawn%20Object%20Reference))
  (Utilities|FlowControl|DoOnce false
    (:Completed
      (CallFunction|Open)
      (return true))))