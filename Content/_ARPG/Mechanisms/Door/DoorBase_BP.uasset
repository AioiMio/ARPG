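; Base door actor that a pawn interacts with to open it once, swinging the mesh open with a timeline and playing a sound.
; Interact allows one-sided doors, checked by a dot product against the forward vector, and an optional required gameplay tag on the instigator's ability system component.
; A refused interaction sets a failure message, such as locked or wrong side, and returns false.
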(event Custom|Open
  (Variables|Default|SetbTriggered true)
  (Utilities|FlowControl|Sequence
    (:then_0
      (bind _alpha (Timeline|Timeline_Open PlayFromStart)
        (:Update
          (Transformation|SetRelativeRotation (Variables|Default|GetBaseMesh) (Math|Rotator|MakeRotator 0.0 0.0 (Math|Float|Lerp 0.0 -9e+01 _alpha)) false false))))
    (:then_1
      (CallFunction|PlaySound))))

(event Custom|PlaySound
  (Audio|PlaySoundatLocation (Variables|Default|GetSound) (Transformation|GetActorLocation) "0, 0, 0" 1.0 1.0 0.0 0 0 0 0))

(event EventBeginPlay)

(event Collision|EventActorBeginOverlap
  (params (OtherActor :type Actor%20Object%20Reference)))

(event EventTick
  (params (DeltaSeconds :type Float%20%28single-precision%29)))

(fn ConstructionScript)

(fn Interact
  (params (InstigatorPawn :type Pawn%20Object%20Reference))
  (bind _requiredtag (Variables|Default|GetRequiredTag))
  (if (Variables|Default|GetTwoSide)
    (if (GameplayTags|IsGameplayTagValid _requiredtag) :!label _label
      (if (GameplayTags|HasMatchingGameplayTag (Ability|GetAbilitySystemComponent InstigatorPawn) _requiredtag)
        _
        (else
          (Variables|Default|SetFailedMessage "It's locked")
          (return false))))
    (elif (> (Math|Vector|DotProduct (- (Transformation|GetActorLocation InstigatorPawn) (Transformation|GetActorLocation)) (Transformation|GetActorForwardVector)) 0.0)
      (goto _label)
      (else
        (Variables|Default|SetFailedMessage "Does not open from this side")
        (return false))))
  (Utilities|FlowControl|DoOnce false
    (:Completed
      (CallFunction|Open)
      (return true))))