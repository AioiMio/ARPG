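; Base door Blueprint that a pawn can open once through Interact, swinging its static mesh to -90 degrees yaw.
; Unless TwoSide is set, a dot product against the door's forward vector allows opening only from the front, otherwise setting a failure message.
; A DoOnce guards the Open event, which sets Triggered and drives the rotation with a timeline.
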(event Custom|Open
  (Variables|Default|SetbTriggered true)
  (bind _alpha (Timeline|Timeline_Open PlayFromStart)
    (:Update
      (Transformation|SetRelativeRotation (Variables|Default|GetStaticMeshComponent) (Math|Rotator|MakeRotator 0.0 0.0 (Math|Float|Lerp 0.0 -9e+01 _alpha)) false false))))

(event EventBeginPlay)

(event Collision|EventActorBeginOverlap
  (params (OtherActor :type Actor%20Object%20Reference)))

(event EventTick
  (params (DeltaSeconds :type Float%20%28single-precision%29)))

(fn ConstructionScript)

(fn Interact
  (params (InstigatorPawn :type Pawn%20Object%20Reference))
  (if (Variables|Default|GetTwoSide)
    _
    (elif (> (Math|Vector|DotProduct (- (Transformation|GetActorLocation InstigatorPawn) (Transformation|GetActorLocation)) (Transformation|GetActorForwardVector)) 0.0)
      _
      (else
        (Variables|Default|SetFailedMessage "Does not open from this side")
        (return false))))
  (Utilities|FlowControl|DoOnce false
    (:Completed
      (CallFunction|Open)
      (return true))))