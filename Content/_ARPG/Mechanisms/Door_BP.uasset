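; Interactable door Blueprint that swings open once when a pawn interacts with it.
; Unless Twoside is set, a dot product against the door's forward vector allows opening only when the instigator stands on the front side.
; A DoOnce gate then calls Open, whose timeline lerps the static mesh's relative yaw through a quarter turn, with no closing logic.
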(event Custom|Open
  (bind _alpha (Timeline|Open_Timeline PlayFromStart)
    (:Update
      (Transformation|SetRelativeRotation (Variables|Default|GetStaticMeshComponent) (Math|Rotator|MakeRotator 0.0 0.0 (Math|Float|Lerp 0.0 -9e+01 _alpha)) false false))))

(event EventBeginPlay)

(event Collision|EventActorBeginOverlap
  (params (OtherActor :type Actor%20Object%20Reference)))

(event EventTick
  (params (DeltaSeconds :type Float%20%28single-precision%29)))

(event EventInteract
  (params (InstigatorPawn :type Pawn%20Object%20Reference))
  (if (Variables|Default|GetTwoside)
    (Utilities|FlowControl|DoOnce false :!label _label
      (:Completed
        (CallFunction|Open)))
    (elif (> (Math|Vector|DotProduct (- (Transformation|GetActorLocation InstigatorPawn) (Transformation|GetActorLocation)) (Transformation|GetActorForwardVector)) 0.0)
      (goto _label))))

(fn ConstructionScript)