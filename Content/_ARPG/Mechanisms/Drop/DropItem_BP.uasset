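; DropItem_BP is an interactable loot drop actor that grants a gameplay effect to whoever picks it up.
; On BeginPlay it maps its Rarity, from Normal to Legendary, to a matching Niagara system and assigns it to the Niagara component.
; Interact marks it triggered, applies GameplayEffectToApply to the instigator pawn's ability system component, then sets a brief lifespan so the actor destroys itself.
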(event EventBeginPlay
  (switch Utilities|FlowControl|Switch|SwitchonEItemRarity (Variables|Default|GetRarity)
    (:Normal
      (Variables|Default|SetPartical "/Game/Assets/sA_ItemDropFx/Fx/NS_Normal_System.NS_Normal_System"))
    (:Uncommon
      (Variables|Default|SetPartical "/Game/Assets/sA_ItemDropFx/Fx/NS_Uncommon_System.NS_Uncommon_System"))
    (:Rare
      (Variables|Default|SetPartical "/Game/Assets/sA_ItemDropFx/Fx/NS_Rare_System.NS_Rare_System"))
    (:Epic
      (Variables|Default|SetPartical "/Game/Assets/sA_ItemDropFx/Fx/NS_Epic_System.NS_Epic_System"))
    (:Mythical
      (Variables|Default|SetPartical "/Game/Assets/sA_ItemDropFx/Fx/NS_Mythical_System.NS_Mythical_System"))
    (:Legendary
      (Variables|Default|SetPartical "/Game/Assets/sA_ItemDropFx/Fx/NS_Legendary_System.NS_Legendary_System")))
  (Class|NiagaraComponent|SetAsset (Variables|Default|GetNiagara) (Variables|Default|GetPartical) true))

(event Collision|EventActorBeginOverlap
  (params (OtherActor :type Actor%20Object%20Reference)))

(event EventTick
  (params (DeltaSeconds :type Float%20%28single-precision%29)))

(fn ConstructionScript)

(fn Interact
  (params (InstigatorPawn :type Pawn%20Object%20Reference))
  (Variables|Default|SetbTriggered true)
  (GameplayEffects|ApplyGameplayEffectToSelf :self (Ability|GetAbilitySystemComponent InstigatorPawn) :GameplayEffectClass (Variables|Interact|GetGameplayEffectToApply))
  (Actor|SetLifeSpan 0.1)
  (return false))