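; Interactable wall mechanism that topples over when a pawn uses it from the side its forward vector faces.
; Interact checks that side with a dot product, then calls Fall through a DoOnce and returns true; it returns false from the other side.
; Fall sets Triggered, pitches BaseMesh over with a timeline-driven lerp, and plays an attenuated interaction sound followed by a delayed stone explosion.
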(event Custom|Fall
  (Variables|Default|SetbTriggered true)
  (Utilities|FlowControl|Sequence
    (:then_0
      (bind _alpha (Timeline|Timeline_Fall PlayFromStart)
        (:Update
          (Transformation|SetRelativeRotation (Variables|Default|GetBaseMesh) (Math|Rotator|MakeRotator 0.0 (Math|Float|Lerp 0.0 107.0 _alpha) 0.0) false false))))
    (:then_1
      (CallFunction|PlaySound "/Game/Assets/ARPG_Weapon_Sounds/WAV/Bow/Bow_interaction_1.Bow_interaction_1")
      (Utilities|FlowControl|Delay 1.0)
      (CallFunction|PlaySound "/Game/Assets/Combat_Sounds_Bundle_Collection/WAV/With_Echo/Object_Destruction/Stones_Explosion_02_With_Echo_Enhancement.Stones_Explosion_02_With_Echo_Enhancement"))))

(event Custom|PlaySound
  (params (Sound :type Sound%20Base%20Object%20Reference))
  (Audio|PlaySoundatLocation Sound (Transformation|GetActorLocation) "0, 0, 0" 1.0 1.0 0.0 "/Game/_ARPG/Sounds/Attenuations/AttenuationBase.AttenuationBase" 0 0 0))

(event EventBeginPlay)

(event Collision|EventActorBeginOverlap
  (params (OtherActor :type Actor%20Object%20Reference)))

(event EventTick
  (params (DeltaSeconds :type Float%20%28single-precision%29)))

(fn ConstructionScript)

(fn Interact
  (params (InstigatorPawn :type Pawn%20Object%20Reference))
  (if (> (Math|Vector|DotProduct (- (Transformation|GetActorLocation InstigatorPawn) (Transformation|GetActorLocation)) (Transformation|GetActorForwardVector)) 0.0)
    (Utilities|FlowControl|DoOnce false
      (:Completed
        (CallFunction|Fall)
        (return true)))
    (else
      (return false))))