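; Fog gate mechanism that acts as a one-way passage, moving the interacting pawn through to a set exit point.
; Interact uses a dot product against the gate's forward vector to accept only pawns on the front side, and a DoOnce limits it to a single use.
; Traverse instantly sets the pawn's location and rotation to those of the Billboard component, which marks the destination.
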(event EventBeginPlay)

(event Collision|EventActorBeginOverlap
  (params (OtherActor :type Actor%20Object%20Reference)))

(event EventTick
  (params (DeltaSeconds :type Float%20%28single-precision%29)))

(fn ConstructionScript)

(fn Interact
  (params (InstigatorPawn :type Pawn%20Object%20Reference))
  (if (> (Math|Vector|DotProduct (- (Transformation|GetActorLocation InstigatorPawn) (Transformation|GetActorLocation)) (Transformation|GetActorForwardVector)) 0.0)
    (Utilities|FlowControl|DoOnce false
      (:Completed
        (CallFunction|Traverse InstigatorPawn)
        (return true)))
    (else
      (return false))))

(fn Traverse
  (params (Instigator :type Actor%20Object%20Reference))
  (bind _billboard (Variables|Default|GetBillboard))
  (Transformation|SetActorLocationAndRotation Instigator (Transformation|GetWorldLocation _billboard) (Transformation|GetWorldRotation _billboard)))