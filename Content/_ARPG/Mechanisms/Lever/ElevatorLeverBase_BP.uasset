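; Base lever that a pawn interacts with to trigger a linked elevator.
; Interaction is allowed only while untriggered and the elevator's position matches TriggerCondition.
; Pulling plays a sound and a timeline that rolls the additive mesh, then calls TriggerDown on the target.
; The target's OnTargetReached event reverses the rotation through a second timeline and clears the triggered flag.
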(event Custom|Pull
  (bind _target (Variables|Default|GetTarget))
  (Variables|Default|SetbTriggered true)
  (Utilities|FlowControl|Sequence
    (:then_0
      (bind _alpha (Timeline|Timeline_Pull PlayFromStart)
        (:Update
          (Transformation|SetRelativeRotation (Variables|Default|GetAdditiveMesh) (Math|Rotator|MakeRotator (Math|Float|Lerp 0.0 -9e+01 _alpha) 0.0 0.0) false false))
        (:Finished
          (Utilities|IsValid _target
            (:Is%20Valid
              (Default|TriggerDown _target))))))
    (:then_1
      (CallFunction|PlaySound))))

(event Custom|PlaySound
  (Audio|PlaySoundatLocation (Variables|Default|GetSound) (Transformation|GetActorLocation) "0, 0, 0" 0.5 1.0 0.0 0 0 0 0))

(event Custom|OnTargetReached
  (CallFunction|ResetTrigger))

(event Custom|ResetTrigger
  (if (Variables|Default|GetbTriggered)
    (bind _alpha (Timeline|Timeline_ResetTrigger ReverseFromEnd)
      (:Update
        (Transformation|SetRelativeRotation (Variables|Default|GetAdditiveMesh) (Math|Rotator|MakeRotator (Math|Float|Lerp 0.0 -9e+01 _alpha) 0.0 0.0) false false))
      (:Finished
        (Variables|Default|SetbTriggered false)))))

(event EventBeginPlay
  (EventDispatchers|AssignOnTargetReached (Variables|Default|GetTarget) (delegate Custom|OnTargetReached)))

(fn ConstructionScript)

(fn Interact
  (params (InstigatorPawn :type Pawn%20Object%20Reference))
  (Utilities|FlowControl|DoOnce false
    (:Completed
      (CallFunction|Pull)
      (return true))))

(fn CanInteract
  (params (InstigatorPawn :type Pawn%20Object%20Reference))
  (return (and (not (Variables|Default|GetbTriggered)) (Utilities|Enum|Equal(Enum) (Variables|/Game/_ARPG/Mechanisms/Target/ElevatorBase_BP.ElevatorBase_BP_C|GetElevatorPosition (Variables|Default|GetTarget)) (Variables|Default|GetTriggerCondition)))))