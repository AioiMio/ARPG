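; Base lever mechanism that a pawn can pull once through Interact to operate an assigned Target.
; Pulling sets Triggered, plays a sound at the lever and runs a timeline that rolls the additive mesh through a quarter turn.
; When the animation finishes, the lever sends OperateMessage to Target if it is valid and implements BPI_Operate.
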(event Custom|Pull
  (bind _target (Variables|Default|GetTarget))
  (Variables|Default|SetbTriggered true)
  (Utilities|FlowControl|Sequence
    (:then_0
      (bind _alpha (Timeline|Timeline_Pull PlayFromStart)
        (:Update
          (Transformation|SetRelativeRotation (Variables|Default|GetAdditiveMesh) (Math|Rotator|MakeRotator (Math|Float|Lerp 0.0 -9e+01 _alpha) 0.0 0.0) false false))
        (:Finished
          (Utilities|IsValid _target
            (:Is%20Valid
              (if (Utilities|DoesObjectImplementInterface _target "/Game/_ARPG/Mechanisms/Target/BPI_Operate.BPI_Operate_C")
                (Class|BPIOperate|Operate(Message) _target)))))))
    (:then_1
      (CallFunction|PlaySound))))

(event Custom|PlaySound
  (Audio|PlaySoundatLocation (Variables|Default|GetSound) (Transformation|GetActorLocation) "0, 0, 0" 0.5 1.0 0.0 0 0 0 0))

(event EventBeginPlay)

(event Collision|EventActorBeginOverlap
  (params (OtherActor :type Actor%20Object%20Reference)))

(event EventTick
  (params (DeltaSeconds :type Float%20%28single-precision%29)))

(fn ConstructionScript)

(fn Interact
  (params (InstigatorPawn :type Pawn%20Object%20Reference))
  (Utilities|FlowControl|DoOnce false
    (:Completed
      (CallFunction|Pull)
      (return true))))