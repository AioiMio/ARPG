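; BridgeBase_BP is a bridge mechanism target that rises vertically when operated.
; BeginPlay caches its starting location, and Operate plays a timeline that lerps the actor's Z upward from that point by a fixed height.
; A metal sound plays as the lift starts and another when it finishes, both through a shared PlaySound event at the actor's position.
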(event Custom|PlaySound
  (params (Sound :type Sound%20Wave%20Object%20Reference))
  (Audio|PlaySoundatLocation Sound (Transformation|GetActorLocation) "0, 0, 0" 0.5 1.0 0.0 0 0 0 0))

(event EventBeginPlay
  (Variables|Default|SetDefaultLocation (Transformation|GetActorLocation)))

(event Collision|EventActorBeginOverlap
  (params (OtherActor :type Actor%20Object%20Reference)))

(event EventTick
  (params (DeltaSeconds :type Float%20%28single-precision%29)))

(event EventOperate
  (bind _defaultlocation (Variables|Default|GetDefaultLocation))
  (Utilities|FlowControl|Sequence
    (:then_0
      (bind _alpha (Timeline|Timeline_Lift PlayFromStart)
        (:Update
          (Transformation|SetActorLocation (Math|Vector|MakeVector (.x _defaultlocation) (.y _defaultlocation) (+ (.z _defaultlocation) (Math|Float|Lerp 0.0 1.8e+03 _alpha))) false false))
        (:Finished
          (CallFunction|PlaySound "/Game/Assets/metal_interactions/metal_interaction2.metal_interaction2"))))
    (:then_1
      (CallFunction|PlaySound "/Game/Assets/metal_interactions/metal_interaction1.metal_interaction1"))))

(fn ConstructionScript)