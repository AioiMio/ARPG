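; Base elevator platform that travels between its start location and a relative target offset when an ARPGCharacter stands on its trigger.
; On authority, the trigger box runs a confirmation timeline and, if a character still overlaps, animates the button down and calls Operate.
; Operate plays or reverses a lift timeline that lerps the actor between endpoints, with sounds.
; On arrival it updates the position, re-arms the button and calls OnTargetReached.
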(event OnComponentBeginOverlap(TriggerBox)
  (params (OverlappedComponent :type Primitive%20Component%20Object%20Reference) (OtherActor :type Actor%20Object%20Reference) (OtherComp :type Primitive%20Component%20Object%20Reference) (OtherBodyIndex :type Integer) (bFromSweep :type Boolean) (SweepResult :type Hit%20Result%20Structure%20%28by%20ref%29))
  (Networking|SwitchHasAuthority
    (:Authority
      (if (Variables|Default|GetCanTrigger)
        (Utilities|Casting|CastToARPGCharacter OtherActor)
        (Utilities|FlowControl|DoOnce false :!label _label
          (:Completed
            (Timeline|Timeline_WaitConfirm PlayFromStart
              (:Finished
                (Utilities|FlowControl|Sequence
                  (:then_0
                    (if (> (Utilities|Array|Length (Collision|GetOverlappingActors (Variables|Default|GetTriggerBox) "/Script/ARPG.ARPGCharacter" :!class /Script/Engine.PrimitiveComponent)) 0)
                      (CallFunction|TriggerDown)))
                  (:then_1
                    (goto _label Reset)))))))))))

(event Custom|ResetTrigger
  (bind _alpha (Timeline|Timeline_ResetTrigger PlayFromStart)
    (:Update
      (Transformation|SetRelativeLocation (Variables|Default|GetTrigger) (Math|Vector|MakeVector 0.0 (- (.y (Variables|Default|GetDefaultTriggerLocation)) (Math|Float|Lerp 0.0 3.0 _alpha)) 0.0) false false))
    (:Finished
      (Variables|Default|SetCanTrigger true))))

(event Custom|PlaySound
  (params (Sound :type Sound%20Wave%20Object%20Reference))
  (Audio|PlaySoundatLocation Sound (Transformation|GetActorLocation) "0, 0, 0" 0.5 1.0 0.0 0 0 0 0))

(event Custom|TriggerDown
  (Variables|Default|SetCanTrigger false)
  (bind _alpha (Timeline|Timeline_Button PlayFromStart)
    (:Update
      (Transformation|SetRelativeLocation (Variables|Default|GetTrigger) (Math|Vector|MakeVector 0.0 (- (.y (Variables|Default|GetDefaultTriggerLocation)) (Math|Float|Lerp 0.0 3.0 _alpha)) 0.0) false false))
    (:Finished
      (CallFunction|Operate))))

(event EventBeginPlay
  (Variables|Default|SetDefaultLocation (Transformation|GetActorLocation))
  (Variables|Default|SetDefaultTriggerLocation (Variables|/Script/Engine.SceneComponent|GetRelativeLocation (Variables|Default|GetTrigger)))
  (Variables|Default|SetTargetLocation (+ (Math|Vector|RotateVector (* (Variables|Default|GetTargetRelativeLocation) (Transformation|GetActorScale3D)) (Transformation|GetActorRotation)) (Variables|Default|GetDefaultLocation))))

(event Collision|EventActorBeginOverlap
  (params (OtherActor :type Actor%20Object%20Reference)))

(event EventTick
  (params (DeltaSeconds :type Float%20%28single-precision%29)))

(event EventOperate
  (Utilities|FlowControl|Sequence
    (:then_0
      (if (Utilities|Enum|Equal(Enum) (Variables|Default|GetElevatorPosition) "Down")
        (Variables|Default|SetTargetPosition "Up")
        (Variables|Default|SetElevatorPosition "None")
        (bind _alpha (Timeline|Timeline_Lift PlayFromStart)
          (:Update
            (Transformation|SetActorLocation (Math|Vector|Lerp(Vector) (Variables|Default|GetDefaultLocation) (Variables|Default|GetTargetLocation) _alpha) false false))
          (:Finished
            (CallFunction|PlaySound "/Game/Assets/metal_interactions/metal_interaction2.metal_interaction2")
            (Variables|Default|SetElevatorPosition (Variables|Default|GetTargetPosition))
            (CallFunction|ResetTrigger)
            (Default|CallOnTargetReached)))
        (elif (Utilities|Enum|Equal(Enum) (Variables|Default|GetElevatorPosition) "Up")
          (Variables|Default|SetTargetPosition "Down")
          (Variables|Default|SetElevatorPosition "None")
          (Timeline|Timeline_Lift ReverseFromEnd))))
    (:then_1
      (CallFunction|PlaySound "/Game/Assets/metal_interactions/metal_interaction1.metal_interaction1"))))

(fn ConstructionScript)